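; BP_Tree is a tree actor that switches between living and dead states as part of a revive-trees task.
; The TaskReviveTrees event sets whether it is active, and only then does its sphere overlap check for projectiles.
; BP_Projectile revives a dead tree and increments the BP_NPC_ReviveTrees counter, while BP_EnemyProjectile kills a living one.
; Each state change swaps the static mesh, with snowy variants chosen by IsSnowy.
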(event `self.ReceiveBeginPlay`)

(event `/Game/Systems/Blueprint/Interfaces/BPI_NPCTaskManager.Task_ReviveTrees`
  (params (`IsActive?` :type Boolean))
  ;[1 1 1] Activates Task
  (set `self.Is Active?` `IsActive?`))

(event `self.Sphere.OnComponentBeginOverlap`
  (params (OverlappedComponent :type "PrimitiveComponent Object Reference") (OtherActor :type "Actor Object Reference") (OtherComp :type "PrimitiveComponent Object Reference") (OtherBodyIndex :type Integer) (bFromSweep :type Boolean) (SweepResult :type "HitResult Structure (by ref)"))
  (bind _isdead_ (`self.IsDead?`))
  (bind _staticmesh (`self.StaticMesh`))
  (bind _staticmesh_2 (`self.StaticMesh`))
  (if (`self.Is Active?`)
    (if (> (`KismetArrayLibrary.Array_Length` (`PrimitiveComponent.GetOverlappingActors` (`self.Sphere`) "/Game/Systems/Blueprint/BP_Projectile.BP_Projectile_C")) 0)
      (if _isdead_
        (set `self.IsDead?` false)
        (if (`self.IsSnowy?`)
          (`StaticMeshComponent.SetStaticMesh` _staticmesh "/Game/Systems/Meshes/DownloadedMeshes/150LowPolyNatureModels/CommonTree_Snow_1.CommonTree_Snow_1")
          (else
            (`StaticMeshComponent.SetStaticMesh` _staticmesh "/Game/Systems/Meshes/DownloadedMeshes/150LowPolyNatureModels/CommonTree_1.CommonTree_1")))
        (bind _returnvalue (`GameplayStatics.GetActorOfClass` "/Game/Systems/Blueprint/myCharacters/NPCs/BP_NPC_ReviveTrees.BP_NPC_ReviveTrees_C"))
        (bind _result (`/Engine/EditorBlueprintResources/StandardMacros.IncrementInt` (`/Game/Systems/Blueprint/myCharacters/NPCs/BP_NPC_ReviveTrees.RevivedCounter` _returnvalue))
          (:`  `
            (`KismetSystemLibrary.PrintString` (`KismetStringLibrary.Conv_IntToString` _result)))))
      (elif (> (`KismetArrayLibrary.Array_Length` (`PrimitiveComponent.GetOverlappingActors` (`self.Sphere`) "/Game/Systems/Blueprint/myCharacters/Enemy/BP_EnemyProjectile.BP_EnemyProjectile_C")) 0)
        (if (not _isdead_)
          (set `self.IsDead?` true)
          (if (`self.IsSnowy?`)
            (`StaticMeshComponent.SetStaticMesh` _staticmesh_2 "/Game/Systems/Meshes/DownloadedMeshes/150LowPolyNatureModels/CommonTree_Dead_Snow_1.CommonTree_Dead_Snow_1")
            (else
              (`StaticMeshComponent.SetStaticMesh` _staticmesh_2 "/Game/Systems/Meshes/DownloadedMeshes/150LowPolyNatureModels/CommonTree_Dead_1.CommonTree_Dead_1"))))))))

(event `self.StaticMesh.OnComponentHit`
  (params (HitComponent :type "PrimitiveComponent Object Reference") (OtherActor :type "Actor Object Reference") (OtherComp :type "PrimitiveComponent Object Reference") (NormalImpulse :type "Vector Structure") (Hit :type "HitResult Structure (by ref)")))

(event `self.StaticMesh.OnComponentBeginOverlap`
  (params (OverlappedComponent :type "PrimitiveComponent Object Reference") (OtherActor :type "Actor Object Reference") (OtherComp :type "PrimitiveComponent Object Reference") (OtherBodyIndex :type Integer) (bFromSweep :type Boolean) (SweepResult :type "HitResult Structure (by ref)")))

(fn `UserConstructionScript`)