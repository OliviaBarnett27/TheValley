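; BP_Wheelbarrow is a wheelbarrow actor that attaches to the player and visibly fills with debris.
; At BeginPlay it stores its location and hides nine debris components.
; Overlapping HandleCollision attaches it to the player character; each Frontcollision overlap reveals the next piece if the actor overlaps a BP_DebrisPile.
; On destruction it prints debug text and, after a validity check, spawns a replacement at the stored location.
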(event `self.ReceiveBeginPlay`
  (set `self.OriginLocation` (`SceneComponent.K2_GetComponentLocation` (`self.Body`)))
  (bind _debrisarray (`self.Create Debris Array`))
  (bind _output_get (set `self.Debris Array` _debrisarray))
  (for _array_element _output_get
    (`SceneComponent.SetHiddenInGame` _array_element true false)))

(event `self.HandleCollision.OnComponentBeginOverlap`
  (params (OverlappedComponent :type "PrimitiveComponent Object Reference") (OtherActor :type "Actor Object Reference") (OtherComp :type "PrimitiveComponent Object Reference") (OtherBodyIndex :type Integer) (bFromSweep :type Boolean) (SweepResult :type "HitResult Structure (by ref)"))
  ;[1 1 1] Attaches to player character
  (`self.K2_AttachToActor` (`GameplayStatics.GetPlayerCharacter` 0) "None" "KeepWorld" "KeepWorld" "KeepWorld"))

(event `self.ReceiveDestroyed`
  (`KismetSystemLibrary.PrintString` "?????????")
  (`/Engine/EditorBlueprintResources/StandardMacros.IsValid` null
    (:`Is Valid`
      (`KismetSystemLibrary.PrintString` "??? BUT AGAIN")
      (`|SpawnActorFromClass` "BP_Wheelbarrow_C" (`KismetMathLibrary.MakeTransform` (`self.OriginLocation`) (`self.OriginRotation`)) "Undefined" "MultiplyWithRoot" null null))))

(event `self.frontcollision.OnComponentBeginOverlap`
  (params (OverlappedComponent :type "PrimitiveComponent Object Reference") (OtherActor :type "Actor Object Reference") (OtherComp :type "PrimitiveComponent Object Reference") (OtherBodyIndex :type Integer) (bFromSweep :type Boolean) (SweepResult :type "HitResult Structure (by ref)"))
  (bind _index (`self.Index`))
  (if (> (`KismetArrayLibrary.Array_Length` (`self.GetOverlappingActors` "/Game/Systems/Blueprint/BP_DebrisPile.BP_DebrisPile_C")) 0)
    (`SceneComponent.SetHiddenInGame` (`|GetArrayItem` (`self.Debris Array`) _index) false false)
    (`/Engine/EditorBlueprintResources/StandardMacros.IncrementInt` _index)))

(fn `Create Debris Array`
  (returns (DebrisArray :type "Array of StaticMeshComponent Object Reference"))
  (return (`|MakeArray` (`self.Debris0`) (`self.Debris1`) (`self.Debris2`) (`self.Debris3`) (`self.Debris4`) (`self.Debris5`) (`self.Debris6`) (`self.Debris7`) (`self.Debris8`))))

(fn `UserConstructionScript`)