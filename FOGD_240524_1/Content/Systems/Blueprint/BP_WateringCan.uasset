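; BP_WateringCan is a watering can actor that continuously emits BP_WaterDroplet actors.
; Half a second after BeginPlay, it starts a fast looping timer that passes an array of nine Arrow components to SpawnDroplet.
; Each tick of that timer spawns one droplet at the world location of a randomly picked arrow, so the arrows act as scattered emission points.
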(event `self.ReceiveBeginPlay`
  ;[1 1 1] Droplets are spawned every 0.02 seconds
  (`KismetSystemLibrary.Delay` 0.5)
  (`KismetSystemLibrary.K2_SetTimerDelegate` (delegate `WaterDropletTimer`) 0.02 true))

(event `WaterDropletTimer`
  ;[1 1 1] Droplets are spawned every 0.02 seconds
  (`self.Spawn Droplet` (`|MakeArray` (`self.Arrow`) (`self.Arrow1`) (`self.Arrow2`) (`self.Arrow3`) (`self.Arrow4`) (`self.Arrow5`) (`self.Arrow6`) (`self.Arrow7`) (`self.Arrow8`))))

(event `Spawn Droplet`
  (params (Arrow :type "Array of ArrowComponent Object Reference"))
  ;[1 1 1] Spawns a droplet at the position of a random arrow
  (`|SpawnActorFromClass` "/Game/Systems/Blueprint/BP_WaterDroplet.BP_WaterDroplet_C" (`KismetMathLibrary.MakeTransform` (`SceneComponent.K2_GetComponentLocation` (`KismetArrayLibrary.Array_Random` Arrow))) "Undefined" "MultiplyWithRoot" null null))

(fn `UserConstructionScript`)