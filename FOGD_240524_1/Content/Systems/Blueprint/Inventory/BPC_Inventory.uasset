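; BPC_Inventory is an inventory component that keeps a list of item names and mirrors changes to a WBP_Inventory widget.
; Add and remove functions update the array and message the widget it creates, though UI removal always passes index 0.
; LevelChange copies the array to MyGameInstance and prints it, and LoadInventory re-adds those saved items, carrying inventory across levels.
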(event `/Game/Systems/Blueprint/Interfaces/BPI_LevelChange.LevelChange`
  (bind _asmy_game_instance (cast `/Game/Systems/MyGameInstance` (`GameplayStatics.GetGameInstance`)))
  (bind _output_get (set `/Game/Systems/MyGameInstance.InventoryGI` (`self.Inventory`) _asmy_game_instance))
  (for _array_element _output_get
    (`KismetSystemLibrary.PrintString` _array_element)))

(event `/Game/Systems/Blueprint/Interfaces/BPI_Trail.LoadInventory`
  (bind _asmy_game_instance (cast `/Game/Systems/MyGameInstance` (`GameplayStatics.GetGameInstance`)))
  (for _array_element (`/Game/Systems/MyGameInstance.InventoryGI` _asmy_game_instance)
    (`self.Add Item To Inventory` _array_element)))

(fn `Add Item To Inventory`
  (params (ItemName :type "String (by ref)") (Actor :type "Object Object Reference"))
  (`KismetArrayLibrary.Array_Add` (`self.Inventory`) ItemName)
  (message `/Game/Systems/Blueprint/Interfaces/BPI_NewPickUp.AddItemToUIList` (`self.WBP Inventory`) ItemName))

(fn `CreateWidget`
  (returns (`WBP Inventory` :type "/Game/Systems/UI/WBP_Inventory Object Reference"))
  (bind _returnvalue (`|CreateWidget` "/Game/Systems/UI/WBP_Inventory.WBP_Inventory_C"))
  (bind _output_get (set `self.WBP Inventory` _returnvalue))
  (return _output_get))

(fn `GetInventory`
  (returns (NewParam :type "Array of String"))
  (return))

(fn `RemoveItemFromInventory`
  (params (ItemsConsumed :type Integer) (PlayerCharacter :type "/Game/Systems/PlayerCharacter/PlayerCharacter/BP_PlayerCharacter Object Reference"))
  (`KismetArrayLibrary.Array_Remove` (`self.Inventory`) ItemsConsumed)
  (message `/Game/Systems/Blueprint/Interfaces/BPI_NewPickUp.RemoveItemFromUIList` (`self.WBP Inventory`) 0 PlayerCharacter)
  (set `self.GIInventory` (`self.Inventory`)))