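; BPC_Dialogue is a dialogue component Blueprint meant to show lines from a Dialogue array as a speech bubble on the player's HUD.
; Its Speak event takes start and end lines but is empty, leaving the display logic disconnected so it never runs.
; That orphaned logic swaps the bubble into the HUD's SpeechHolder, checks line bounds, then clears it after a retriggerable delay and prints a completion message.
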(event `Speak`
  (params (StartLine :type Integer) (EndLine :type Integer)))