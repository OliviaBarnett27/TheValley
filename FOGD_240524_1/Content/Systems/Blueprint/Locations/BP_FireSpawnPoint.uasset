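; BP_FireSpawnPoint is a fire hazard for a put-out-fires task, dormant until that task event switches it on.
; The event sets IsActive and starts the Niagara fire effect, which is deactivated at BeginPlay.
; While active, it deals fixed damage to actors that begin overlapping its capsule.
; Damage it receives while active drains Health, and it destroys itself when Health runs out.
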(event `self.ReceiveBeginPlay`
  (`ActorComponent.Deactivate` (`self.FireNiagara`)))

(event `/Game/Systems/Blueprint/Interfaces/BPI_NPCTaskManager.Task_PutOutFires`
  (params (`IsActive?` :type Boolean))
  (bind _output_get (set `self.IsActive?` `IsActive?`))
  (if _output_get
    (`ActorComponent.Activate` (`self.FireNiagara`) false)))

(event `self.ReceiveAnyDamage`
  (params (Damage :type "Float (single-precision)") (DamageType :type "DamageType Object Reference") (InstigatedBy :type "Controller Object Reference") (DamageCauser :type "Actor Object Reference"))
  (if (`self.IsActive?`)
    (bind _output_get (set `self.Health` (- (`self.Health`) Damage)))
    (if (<= _output_get 0.0)
      (`self.K2_DestroyActor`))))

(event `self.Capsule.OnComponentBeginOverlap`
  (params (OverlappedComponent :type "PrimitiveComponent Object Reference") (OtherActor :type "Actor Object Reference") (OtherComp :type "PrimitiveComponent Object Reference") (OtherBodyIndex :type Integer) (bFromSweep :type Boolean) (SweepResult :type "HitResult Structure (by ref)"))
  (if (`self.IsActive?`)
    (`GameplayStatics.ApplyDamage` OtherActor 30.0)))

(fn `UserConstructionScript`)