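; A flower growth spot for a grow-flowers task, where a damageable marker turns into a snowdrop or grass.
; Its cylinder starts hidden and is revealed when the TaskGrowFlowers event fires as active.
; While visible, damage drains Health; at zero it plays a Niagara spawn effect, spawns BP_Snowdrop or BP_Grass by flag with random yaw, and destroys itself.
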(event `/Game/Systems/Blueprint/Interfaces/BPI_NPCTaskManager.Task_GrowFlowers`
  (params (`IsActive?` :type Boolean))
  ;[1 1 1] Reveals all growth spots in world when the task has been activated
  (if `IsActive?`
    (`SceneComponent.SetHiddenInGame` (`self.Cylinder`) false false)
    (set `self.IsHidden?` false)))

(event `self.ReceiveBeginPlay`
  ;[1 1 1] Makes actors hidden from the beginning
  (`SceneComponent.SetHiddenInGame` (`self.Cylinder`) true false)
  (set `self.IsHidden?` true))

(event `self.ReceiveAnyDamage`
  (params (Damage :type "Float (single-precision)") (DamageType :type "DamageType Object Reference") (InstigatedBy :type "Controller Object Reference") (DamageCauser :type "Actor Object Reference"))
  ;[1 1 1] Take Damage
  (if (not (`self.IsHidden?`))
    (bind _output_get (set `self.Health` (- (`self.Health`) Damage)))
    (if (<= _output_get 0.0)
      (if (`self.SpawnSnowdrop?`)
        (`self.Spawn Snowdrop`)
        (elif (`self.SpawnGrass?`)
          (`self.SpawnGrass`))))))

(event `Spawn Snowdrop`
  (bind _returnvalue (`self.K2_GetActorLocation`))
  ;[1 1 1] Spawn Snowdrop
  (`NiagaraFunctionLibrary.SpawnSystemAtLocation` "/Game/Systems/Niagara/NS_Spawn.NS_Spawn" _returnvalue)
  (`|SpawnActorFromClass` "/Game/Systems/Blueprint/Decor/BP_Snowdrop.BP_Snowdrop_C" (`KismetMathLibrary.MakeTransform` _returnvalue (`KismetMathLibrary.MakeRotator` 0.0 0.0 (`KismetMathLibrary.RandomFloatInRange` 0.0 360.0))) "Undefined" "MultiplyWithRoot" null null)
  (`self.K2_DestroyActor`))

(event `SpawnGrass`
  (bind _returnvalue (`self.K2_GetActorLocation`))
  ;[1 1 1] SpawnGrass
  (`NiagaraFunctionLibrary.SpawnSystemAtLocation` "/Game/Systems/Niagara/NS_Spawn.NS_Spawn" _returnvalue)
  (`|SpawnActorFromClass` "/Game/Systems/Blueprint/Decor/BP_Grass.BP_Grass_C" (`KismetMathLibrary.MakeTransform` _returnvalue (`KismetMathLibrary.MakeRotator` 0.0 0.0 (`KismetMathLibrary.RandomFloatInRange` 0.0 360.0))) "Undefined" "MultiplyWithRoot" null null)
  (`self.K2_DestroyActor`))

(fn `UserConstructionScript`)