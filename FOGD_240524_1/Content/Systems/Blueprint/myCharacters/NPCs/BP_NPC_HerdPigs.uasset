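; NPC Blueprint that runs a pig-herding task, rewarding the player and spawning a boss once it completes.
; Task messages every BP_Pig to start herding, caches boss spawn points and starts a looping CheckHerded timer.
; CheckHerded increments HerdedAmount for each penned pig without resetting it between checks.
; When the counter reaches the pig count, it stops the timer, updates the player's task, shakes the camera and spawns the boss AI.
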(event `self.Task`
  (bind _outactors (`GameplayStatics.GetAllActorsOfClass` "/Game/Systems/Blueprint/myCharacters/Pig/BP_Pig.BP_Pig_C"))
  (for _array_element _outactors
    (message `/Game/Systems/Blueprint/Interfaces/BPI_NPCTaskManager.Task_HerdPigs` _array_element true)
    (bind _returnvalue (`KismetSystemLibrary.K2_SetTimerDelegate` (delegate `CheckHerded`) 0.1 true))
    (set `self.CheckingTimer` _returnvalue)
    (bind _outactors_2 (`GameplayStatics.GetAllActorsOfClass` "/Game/Systems/Blueprint/Locations/BP_SpawnPoint_Boss.BP_SpawnPoint_Boss_C"))))

(event `CheckHerded`
  (bind _returnvalue (`GameplayStatics.GetPlayerCameraManager` 0))
  (bind _as_bp_player_character (`self.As BP Player Character`))
  (bind _outactors (`GameplayStatics.GetAllActorsOfClass` "/Game/Systems/Blueprint/myCharacters/Pig/BP_Pig.BP_Pig_C"))
  (for _array_element _outactors
    (if (`/Game/Systems/Blueprint/myCharacters/Pig/BP_Pig.InPen?` _array_element)
      (bind _result (`/Engine/EditorBlueprintResources/StandardMacros.IncrementInt` (`self.HerdedAmount`))
        (:`  `
          (if (>= _result (`KismetArrayLibrary.Array_Length` _outactors))
            (`KismetSystemLibrary.K2_ClearAndInvalidateTimerHandle` (`self.CheckingTimer`))
            (message `/Game/Systems/Blueprint/Interfaces/BPI_NPCTaskManager.GainEnergyForTaskCompletion` _as_bp_player_character 0.0)
            (message `/Game/Systems/Blueprint/Interfaces/BPI_NPCTaskManager.GetActiveTask1` _as_bp_player_character "")
            (`KismetSystemLibrary.Delay` 2.0)
            (bind _returnvalue_2 (`PlayerCameraManager.StartCameraShake` :`self` _returnvalue :`ShakeClass` "/Script/Engine.CameraShakeBase" :`PlaySpace` "World"))
            (`KismetSystemLibrary.Delay` 3.0)
            (`PlayerCameraManager.StopCameraShake` _returnvalue _returnvalue_2 true)
            (`AIBlueprintHelperLibrary.SpawnAIFromClass` "/Game/Systems/Blueprint/myCharacters/Enemy/AI/BP_AIEnemy.BP_AIEnemy_C" "/Game/Systems/Blueprint/myCharacters/Enemy/AI/BT_BossAi.BT_BossAi" (`SceneComponent.K2_GetComponentLocation` (`/Game/Systems/Blueprint/Locations/BP_SpawnPoint_Boss.DefaultSceneRoot` (`|GetArrayItem` (stale `self.Task` _outactors_2)))) (struct) true null)))))))

(fn `UserConstructionScript`
  (`parent.UserConstructionScript`))