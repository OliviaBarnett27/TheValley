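; NPC Blueprint for the put-out-fires task, which leads into the herd-pigs task NPC.
; Task messages every fire spawn point and, inside that loop, sets a looping timer that polls for extinguishing and caches the pig-herder spawn points.
; When no fire spawn point actors remain, the check stops the timer, rewards the player with energy, clears the task box and spawns BP_NPC_HerdPigs at the first cached point.
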(event `self.Task`
  (bind _outactors (`GameplayStatics.GetAllActorsOfClass` "/Game/Systems/Blueprint/Locations/BP_FireSpawnPoint.BP_FireSpawnPoint_C"))
  (for _array_element _outactors
    (message `/Game/Systems/Blueprint/Interfaces/BPI_NPCTaskManager.Task_PutOutFires` _array_element true)
    (bind _returnvalue (`KismetSystemLibrary.K2_SetTimerDelegate` (delegate `Check Extinguished`) 0.5 true))
    (set `self.CheckingTimer` _returnvalue)
    (bind _outactors_2 (`GameplayStatics.GetAllActorsOfClass` "/Game/Systems/Blueprint/Locations/BP_SpawnPoint_HerdPigs.BP_SpawnPoint_HerdPigs_C"))))

(event `Check Extinguished`
  (bind _as_bp_player_character (`self.As BP Player Character`))
  (bind _outactors (`GameplayStatics.GetAllActorsOfClass` "/Game/Systems/Blueprint/Locations/BP_FireSpawnPoint.BP_FireSpawnPoint_C"))
  (if (== (`KismetArrayLibrary.Array_Length` _outactors) 0)
    (`KismetSystemLibrary.K2_ClearAndInvalidateTimerHandle` (`self.CheckingTimer`))
    (message `/Game/Systems/Blueprint/Interfaces/BPI_NPCTaskManager.GainEnergyForTaskCompletion` _as_bp_player_character 200.0)
    (message `/Game/Systems/Blueprint/Interfaces/BPI_NPCTaskManager.GetActiveTask1` _as_bp_player_character "") ; Empties task box
    (`AIBlueprintHelperLibrary.SpawnAIFromClass` "/Game/Systems/Blueprint/myCharacters/NPCs/BP_NPC_HerdPigs.BP_NPC_HerdPigs_C" null (`SceneComponent.K2_GetComponentLocation` (`/Game/Systems/Blueprint/Locations/BP_SpawnPoint_HerdPigs.DefaultSceneRoot` (`|GetArrayItem` (stale `self.Task` _outactors_2)))) (struct) true null)))

(fn `UserConstructionScript`
  (`parent.UserConstructionScript`))