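; BP_NPC_Advice is an NPC Blueprint whose Task event spawns a BP_NPC_BreakIce AI character.
; Task gathers all BP_SpawnPoint_BreakIce actors and runs an empty loop over them.
; A following Sequence branch spawns once at the loop's leftover element location, normally the last spawn point, ignoring collision failure.
; It then prints debug text and the spawn point count.
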(event `self.Task`
  (bind _outactors (`GameplayStatics.GetAllActorsOfClass` "/Game/Systems/Blueprint/Locations/BP_SpawnPoint_BreakIce.BP_SpawnPoint_BreakIce_C"))
  (`|ExecutionSequence`
    (:`then_0`
      (for _array_element _outactors
        _))
    (:`then_1`
      (`AIBlueprintHelperLibrary.SpawnAIFromClass` "/Game/Systems/Blueprint/myCharacters/NPCs/BP_NPC_BreakIce.BP_NPC_BreakIce_C" null (`SceneComponent.K2_GetComponentLocation` (`Actor.RootComponent` _array_element)) (struct) true null)
      (`KismetSystemLibrary.PrintString` "spawn")
      (`KismetSystemLibrary.PrintString` (`KismetStringLibrary.Conv_IntToString` (`KismetArrayLibrary.Array_Length` (`self.Out Actors`)))))))

(fn `UserConstructionScript`
  (`parent.UserConstructionScript`))