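; BP_NPC_MainNPC is an NPC that gives the player a task through dialogue, with an empty Task event as a hook.
; The first player overlap with its interaction collision fires Task and starts Speech, provided the player has no active task.
; Speech re-calls itself on a retriggerable delay to show each dialogue line in the player's HUD speech bubble.
; After the last line, it clears the bubble and passes the task name to the player.
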(event `Task`
  ;[1 1 1] Task
)

(event `self.InteractionCollision.OnComponentBeginOverlap`
  (params (OverlappedComponent :type "PrimitiveComponent Object Reference") (OtherActor :type "Actor Object Reference") (OtherComp :type "PrimitiveComponent Object Reference") (OtherBodyIndex :type Integer) (bFromSweep :type Boolean) (SweepResult :type "HitResult Structure (by ref)"))
  ;[1 1 1] Overlap Trigger
  (bind _asbp_player_character (cast `/Game/Systems/PlayerCharacter/PlayerCharacter/BP_PlayerCharacter` OtherActor))
  (`/Engine/EditorBlueprintResources/StandardMacros.DoOnce` false
    (:`Completed`
      (set `self.As BP Player Character` _asbp_player_character)
      (if (`KismetStringLibrary.EqualEqual_StrStr` (`/Game/Systems/PlayerCharacter/PlayerCharacter/BP_PlayerCharacter.Active Task` (`self.As BP Player Character`)))
        (if true
          (`self.Task`)
          (set `self.Overlapping` false)
          (`self.Speech`))
        (else
          (`KismetSystemLibrary.PrintString` "false"))))))

(event `Speech`
  (bind _as_bp_player_character (`self.As BP Player Character`))
  (bind _speech_bubble (`/Game/Systems/PlayerCharacter/PlayerCharacter/BP_PlayerCharacter.Speech Bubble` _as_bp_player_character))
  (bind _speechholder (`/Game/Systems/UI/WBP_PlayerHUD.SpeechHolder` (`/Game/Systems/PlayerCharacter/PlayerCharacter/BP_PlayerCharacter.PlayerHUD` _as_bp_player_character)))
  ;[1 1 1] Speech
  (`KismetSystemLibrary.PrintString` "child")
  (if (`PanelWidget.HasAnyChildren` _speechholder)
    (`PanelWidget.ClearChildren` _speechholder))
  (set `/Game/Systems/UI/WBP_SpeechBubble.Speech` (`|GetArrayItem` (`self.Dialogue`) (`self.DialogueCounter`)) _speech_bubble)
  (`PanelWidget.AddChild` _speechholder _speech_bubble)
  (`KismetSystemLibrary.RetriggerableDelay` 4.5)
  (bind _result (`/Engine/EditorBlueprintResources/StandardMacros.IncrementInt` (`self.DialogueCounter`))
    (:`  `
      (if (< _result (`KismetArrayLibrary.Array_Length` (`self.Dialogue`)))
        (`self.Speech`)
        (else
          (`PanelWidget.ClearChildren` _speechholder)
          ;[1 1 1] Sets UI textbox to name of task
          (set `self.DialogueCounter` 0)
          (message `/Game/Systems/Blueprint/Interfaces/BPI_NPCTaskManager.GetActiveTask1` (`self.As BP Player Character`) (`self.TaskName`)))))))

(fn `UserConstructionScript`
  (`parent.UserConstructionScript`))