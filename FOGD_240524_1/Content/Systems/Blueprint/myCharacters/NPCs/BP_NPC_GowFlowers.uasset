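; NPC Blueprint for the flower-growing task, which hands off to the tree-revival NPC when finished.
; Its Task event messages every flower growth spot to start the task and sets a looping half-second timer.
; The timer polls until no spots remain, then clears itself, rewards the player energy, empties the task text and spawns BP_NPC_ReviveTrees at the first matching spawn point.
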(event `self.Task`
  ;[1 1 1] Finds every flower growth spot
  (bind _outactors (`GameplayStatics.GetAllActorsOfClass` "/Game/Systems/Blueprint/BP_FlowerGrowthSpot.BP_FlowerGrowthSpot_C"))
  (for _array_element _outactors
    (message `/Game/Systems/Blueprint/Interfaces/BPI_NPCTaskManager.Task_GrowFlowers` _array_element true)
    (bind _returnvalue (`KismetSystemLibrary.K2_SetTimerDelegate` (delegate `CheckDestroyed`) 0.5 true))
    (set `self.CheckingTimer` _returnvalue)
    (bind _outactors_2 (`GameplayStatics.GetAllActorsOfClass` "/Game/Systems/Blueprint/Locations/BP_SpawnPoint_ReviveTrees.BP_SpawnPoint_ReviveTrees_C"))))

(event `CheckDestroyed`
  (bind _as_bp_player_character (`self.As BP Player Character`))
  ;[1 1 1] Clears timer when there are no flower growth spots left
  (bind _outactors (`GameplayStatics.GetAllActorsOfClass` "/Game/Systems/Blueprint/BP_FlowerGrowthSpot.BP_FlowerGrowthSpot_C"))
  (if (== (`KismetArrayLibrary.Array_Length` _outactors) 0)
    (`KismetSystemLibrary.K2_ClearAndInvalidateTimerHandle` (`self.CheckingTimer`))
    (message `/Game/Systems/Blueprint/Interfaces/BPI_NPCTaskManager.GainEnergyForTaskCompletion` _as_bp_player_character 200.0)
    (message `/Game/Systems/Blueprint/Interfaces/BPI_NPCTaskManager.GetActiveTask1` _as_bp_player_character "") ; Empties task box
    ;[1 1 1] Spawn BP_NPC_ReviveTrees
    (`AIBlueprintHelperLibrary.SpawnAIFromClass` "/Game/Systems/Blueprint/myCharacters/NPCs/BP_NPC_ReviveTrees.BP_NPC_ReviveTrees_C" null (`self.K2_GetActorLocation` (`|GetArrayItem` (stale `self.Task` _outactors_2))) (struct) true null)))

(fn `UserConstructionScript`
  (`parent.UserConstructionScript`))