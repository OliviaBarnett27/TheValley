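; Task NPC that gives the player a wheelbarrow job to clear debris piles.
; Task spawns a wheelbarrow with a Niagara effect at the level's wheelbarrow spawn point, then starts a looping timer that polls for remaining debris pile actors.
; When none remain, it stops the timer, rewards the player with energy, clears the active task text and spawns the fires NPC to continue the task chain.
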(event `self.Task`
  (bind _returnvalue (`GameplayStatics.GetActorOfClass` "/Game/Systems/Blueprint/Locations/BP_WheelbarrowSpawnPoint.BP_WheelbarrowSpawnPoint_C"))
  (bind (_returnvalue_location _returnvalue_rotation) (`KismetMathLibrary.BreakTransform` (`SceneComponent.K2_GetComponentToWorld` (`/Game/Systems/Blueprint/Locations/BP_WheelbarrowSpawnPoint.DefaultSceneRoot` _returnvalue))))
  (`NiagaraFunctionLibrary.SpawnSystemAtLocation` "/Game/Systems/Niagara/NS_Spawn.NS_Spawn" _returnvalue_location _returnvalue_rotation)
  (`|SpawnActorFromClass` "/Game/Systems/Blueprint/BP_Wheelbarrow.BP_Wheelbarrow_C" (`KismetMathLibrary.MakeTransform` _returnvalue_location _returnvalue_rotation) "Undefined" "MultiplyWithRoot" null null)
  (bind _returnvalue_2 (`KismetSystemLibrary.K2_SetTimerDelegate` (delegate `CheckCleared`) 0.1 true))
  (set `self.CheckingTimer` _returnvalue_2))

(event `CheckCleared`
  (bind _as_bp_player_character (`self.As BP Player Character`))
  (bind _outactors (`GameplayStatics.GetAllActorsOfClass` "/Game/Systems/Blueprint/BP_DebrisPile.BP_DebrisPile_C"))
  (if (<= (`KismetArrayLibrary.Array_Length` _outactors) 0)
    (`KismetSystemLibrary.K2_ClearAndInvalidateTimerHandle` (`self.CheckingTimer`))
    (message `/Game/Systems/Blueprint/Interfaces/BPI_NPCTaskManager.GainEnergyForTaskCompletion` _as_bp_player_character 100.0)
    (message `/Game/Systems/Blueprint/Interfaces/BPI_NPCTaskManager.GetActiveTask1` _as_bp_player_character "")
    (`AIBlueprintHelperLibrary.SpawnAIFromClass` "/Game/Systems/Blueprint/myCharacters/NPCs/BP_NPC_Fires.BP_NPC_Fires_C" null (`SceneComponent.K2_GetComponentLocation` (`/Game/Systems/Blueprint/Locations/BP_NPCSpawnPoint_Fires.DefaultSceneRoot` (`self.SpawnLocation`))) (struct) true null)))

(fn `UserConstructionScript`
  (`parent.UserConstructionScript`))