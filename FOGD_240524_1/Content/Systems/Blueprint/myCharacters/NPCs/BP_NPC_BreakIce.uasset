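; NPC Blueprint that runs the break-ice task and hands off to the grow-flowers NPC.
; Task fires once, activating every BP_Ice in the level and starting a looping poll timer inside that loop, once per actor.
; When no ice remains, the check clears the last stored timer handle, grants the player energy and clears the task text.
; It then spawns BP_NPC_GowFlowers at the first grow-flowers spawn point.
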(event `self.Task`
  (`/Engine/EditorBlueprintResources/StandardMacros.DoOnce` false
    (:`Completed`
      ;[1 1 1] Activates task for all ice in level
      (bind _outactors (`GameplayStatics.GetAllActorsOfClass` "/Game/Systems/Blueprint/BP_Ice.BP_Ice_C"))
      (for _array_element _outactors
        (message `/Game/Systems/Blueprint/Interfaces/BPI_NPCTaskManager.Task_BreakIce` _array_element true (`self.As BP Player Character`))
        (bind _returnvalue (`KismetSystemLibrary.K2_SetTimerDelegate` (delegate `Check Destroyed Amount`) 0.3 true))
        (set `self.Timer` _returnvalue)
        (bind _outactors_2 (`GameplayStatics.GetAllActorsOfClass` "/Game/Systems/Blueprint/Locations/BP_SpawnPoint_GrowFlowers.BP_SpawnPoint_GrowFlowers_C"))))))

(event `Check Destroyed Amount`
  (bind _as_bp_player_character (`self.As BP Player Character`))
  (bind _outactors (`GameplayStatics.GetAllActorsOfClass` "/Game/Systems/Blueprint/BP_Ice.BP_Ice_C"))
  (if (== (`KismetArrayLibrary.Array_Length` _outactors) 0)
    (`KismetSystemLibrary.K2_ClearAndInvalidateTimerHandle` (`self.Timer`))
    (message `/Game/Systems/Blueprint/Interfaces/BPI_NPCTaskManager.GainEnergyForTaskCompletion` _as_bp_player_character 100.0)
    (message `/Game/Systems/Blueprint/Interfaces/BPI_NPCTaskManager.GetActiveTask1` _as_bp_player_character "")
    ;[1 1 1] Spawn BP_NPC_GrowFlowers
    (`AIBlueprintHelperLibrary.SpawnAIFromClass` "/Game/Systems/Blueprint/myCharacters/NPCs/BP_NPC_GowFlowers.BP_NPC_GowFlowers_C" null (`SceneComponent.K2_GetComponentLocation` (`/Game/Systems/Blueprint/Locations/BP_SpawnPoint_GrowFlowers.DefaultSceneRoot` (`|GetArrayItem` (stale `self.Task` _outactors_2)))) (struct) true null)))

(fn `UserConstructionScript`
  (`parent.UserConstructionScript`))