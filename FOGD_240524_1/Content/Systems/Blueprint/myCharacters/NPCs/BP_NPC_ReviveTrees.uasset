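; NPC Blueprint that runs a tree-revival task for the player.
; Task messages every BP_Tree to enable revival and starts a looping timer that polls whether RevivedCounter equals the tree count.
; On completion it stops the timer, grants the player energy, clears the active task text and spawns a BP_Signpost at the first signpost spawn point.
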(event `self.Task`
  (bind _outactors (`GameplayStatics.GetAllActorsOfClass` "/Game/Systems/Blueprint/BP_Tree.BP_Tree_C"))
  (for _array_element _outactors
    (message `/Game/Systems/Blueprint/Interfaces/BPI_NPCTaskManager.Task_ReviveTrees` _array_element true)
    (bind _returnvalue (`KismetSystemLibrary.K2_SetTimerDelegate` (delegate `Check Revived`) 0.1 true))
    (set `self.CheckingTimer` _returnvalue)
    (bind _outactors_2 (`GameplayStatics.GetAllActorsOfClass` "/Game/Systems/Blueprint/Locations/BP_SpawnPoint_SignPost.BP_SpawnPoint_SignPost_C"))))

(event `Check Revived`
  (bind _as_bp_player_character (`self.As BP Player Character`))
  (if (== (`KismetArrayLibrary.Array_Length` (stale `self.Task` _outactors)) (`self.RevivedCounter`))
    (`KismetSystemLibrary.K2_ClearAndInvalidateTimerHandle` (`self.CheckingTimer`))
    (message `/Game/Systems/Blueprint/Interfaces/BPI_NPCTaskManager.GainEnergyForTaskCompletion` _as_bp_player_character 200.0)
    (message `/Game/Systems/Blueprint/Interfaces/BPI_NPCTaskManager.GetActiveTask1` _as_bp_player_character "")
    (`|SpawnActorFromClass` "/Game/Systems/Blueprint/BP_Signpost.BP_Signpost_C" (`KismetMathLibrary.MakeTransform` (`SceneComponent.K2_GetComponentLocation` (`/Game/Systems/Blueprint/Locations/BP_SpawnPoint_SignPost.DefaultSceneRoot` (`|GetArrayItem` (stale `self.Task` _outactors_2))))) "Undefined" "MultiplyWithRoot" null null)))

(fn `UserConstructionScript`
  (`parent.UserConstructionScript`))