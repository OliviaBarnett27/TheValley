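; Pig character for a herding task that wanders freely, follows the player into a pen, then roams inside it.
; Looping timers drive AIMoveTo in three phases, with random reachable points for free and pen wandering.
; While the task is active, overlapping Detection swaps wandering for following the player, re-issued every 0.1 seconds.
; Each follow tick checks proximity to PenEntrance, which switches the pig to wandering around PenCentre.
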(event `self.ReceiveBeginPlay`
  ;[1 1 1] Free Move
  (bind _returnvalue (`KismetSystemLibrary.K2_SetTimerDelegate` (delegate `FreeMove`) (`KismetMathLibrary.RandomFloatInRange` 2.0 6.0) true))
  (set `self.FreeMoveTimer` _returnvalue))

(event `FreeMove`
  ;[1 1 1] Free Move
  (`|AIMoveTo` self (`NavigationSystemV1.K2_GetRandomReachablePointInRadius` (`self.K2_GetActorLocation`) 1000.0 null null) null 2.0))

(event `/Game/Systems/Blueprint/Interfaces/BPI_NPCTaskManager.Task_HerdPigs`
  (params (`IsActive?` :type Boolean))
  (set `self.Is Active?` `IsActive?`))

(event `self.Detection.OnComponentBeginOverlap`
  (params (OverlappedComponent :type "PrimitiveComponent Object Reference") (OtherActor :type "Actor Object Reference") (OtherComp :type "PrimitiveComponent Object Reference") (OtherBodyIndex :type Integer) (bFromSweep :type Boolean) (SweepResult :type "HitResult Structure (by ref)"))
  (if (`self.Is Active?`)
    (if (not (`self.InPen?`))
      ;[1 1 1] Follow
      (`KismetSystemLibrary.K2_ClearAndInvalidateTimerHandle` (`self.FreeMoveTimer`))
      (set `self.Following?` true)
      (bind _returnvalue (`KismetSystemLibrary.K2_SetTimerDelegate` (delegate `FollowPlayer`) 0.1 true))
      (set `self.FollowMovementTimer` _returnvalue))))

(event `FollowPlayer`
  ;[1 1 1] Follow
  (`|AIMoveTo` self (0.0 0.0 0.0) (`GameplayStatics.GetPlayerCharacter` 0) 100.0
    (:`then`
      ;[1 1 1] Checks if entered pen
      (if (== (`self.K2_GetActorLocation`) (`self.K2_GetActorLocation` (`self.PenEntrance`)) :`ErrorTolerance` 100.0)
        (set `self.InPen?` true)
        (`self.Begin Pen Movement`)))))

(event `Begin Pen Movement`
  ;[1 1 1] Pen Movement
  (if (`self.Following?`)
    (`KismetSystemLibrary.K2_ClearAndInvalidateTimerHandle` (`self.FollowMovementTimer`))
    (set `self.InPen?` true)
    (bind _returnvalue (`KismetSystemLibrary.K2_SetTimerDelegate` (delegate `PenMove`) (`KismetMathLibrary.RandomFloatInRange` 2.0 6.0) true))
    (set `self.PenMovementTimer` _returnvalue)))

(event `PenMove`
  ;[1 1 1] Pen Movement
  (`|AIMoveTo` self (`NavigationSystemV1.K2_GetRandomReachablePointInRadius` (`self.K2_GetActorLocation` (`self.PenCentre`)) 500.0 null null) null 1.0))

(fn `UserConstructionScript`)