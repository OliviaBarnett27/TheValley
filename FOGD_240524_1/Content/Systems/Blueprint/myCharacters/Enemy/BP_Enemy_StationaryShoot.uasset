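; BP_Enemy_StationaryShoot is an enemy that shoots projectiles at the player on detection.
; DetectionSphere begin overlap starts a looping one-second timer that calls Shoot.
; Shoot faces the player, plays the shoot montage and spawns BP_EnemyProjectile at FiringArrow, aimed at the player's current location.
; The timer is cleared when the player ends overlap with CapsuleComponent, not DetectionSphere.
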(event `self.DetectionSphere.OnComponentBeginOverlap`
  (params (OverlappedComponent :type "PrimitiveComponent Object Reference") (OtherActor :type "Actor Object Reference") (OtherComp :type "PrimitiveComponent Object Reference") (OtherBodyIndex :type Integer) (bFromSweep :type Boolean) (SweepResult :type "HitResult Structure (by ref)"))
  (cast `/Game/Systems/PlayerCharacter/PlayerCharacter/BP_PlayerCharacter` OtherActor)
  (bind _returnvalue (`KismetSystemLibrary.K2_SetTimerDelegate` (delegate `Shoot`) 1.0 true))
  (set `self.ShootTimer` _returnvalue))

(event `Shoot`
  (bind _returnvalue (`SceneComponent.K2_GetComponentLocation` (`self.FiringArrow`)))
  (`self.FacePlayer`)
  (`|PlayMontage` null "/Game/Systems/Blueprint/myCharacters/Enemy/AM_Shoot.AM_Shoot"
    (:`then`
      (`|SpawnActorFromClass` "/Game/Systems/Blueprint/myCharacters/Enemy/BP_EnemyProjectile.BP_EnemyProjectile_C" (`KismetMathLibrary.MakeTransform` _returnvalue (`KismetMathLibrary.FindLookAtRotation` _returnvalue (`self.K2_GetActorLocation` (`GameplayStatics.GetPlayerCharacter` 0)))) "Undefined" "MultiplyWithRoot" null null))))

(event `self.CapsuleComponent.OnComponentEndOverlap`
  (params (OverlappedComponent :type "PrimitiveComponent Object Reference") (OtherActor :type "Actor Object Reference") (OtherComp :type "PrimitiveComponent Object Reference") (OtherBodyIndex :type Integer))
  (cast `/Game/Systems/PlayerCharacter/PlayerCharacter/BP_PlayerCharacter` OtherActor)
  (`KismetSystemLibrary.K2_ClearAndInvalidateTimerHandle` (`self.ShootTimer`)))

(fn `UserConstructionScript`
  (`parent.UserConstructionScript`))