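; Boss enemy Blueprint that takes damage and, on death, triggers the player's win message.
; AnyDamage subtracts from Health and zeroes it once it reaches 500 or less, so death occurs at that threshold.
; Death detaches the controller, shakes the camera, starts the death montage, shows the win message and destroys the actor after a delay.
; The capsule's projectile overlap check does nothing, and the Blackboard health update is never executed.
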(event `self.Capsule.OnComponentBeginOverlap`
  (params (OverlappedComponent :type "PrimitiveComponent Object Reference") (OtherActor :type "Actor Object Reference") (OtherComp :type "PrimitiveComponent Object Reference") (OtherBodyIndex :type Integer) (bFromSweep :type Boolean) (SweepResult :type "HitResult Structure (by ref)"))
  (if (> (`KismetArrayLibrary.Array_Length` (`PrimitiveComponent.GetOverlappingActors` (`self.Capsule`) "/Game/Systems/Blueprint/BP_Projectile.BP_Projectile_C")) 0)
    _))

(event `self.ReceiveAnyDamage`
  (params (Damage :type "Float (single-precision)") (DamageType :type "DamageType Object Reference") (InstigatedBy :type "Controller Object Reference") (DamageCauser :type "Actor Object Reference"))
  (`KismetSystemLibrary.PrintString` "hit?")
  (bind _output_get (set `self.Health` (- (`self.Health`) Damage)))
  (if (<= _output_get 500.0)
    (bind _output_get_2 (set `self.Health` 0.0))
    (if (<= _output_get_2 0.0)
      (`self.DetachFromControllerPendingDestroy`)
      (`GameplayStatics.PlayWorldCameraShake` "/Script/Engine.CameraShakeBase" (`SceneComponent.K2_GetComponentLocation` (`self.Mesh`)))
      (`|PlayMontage` null "/Game/Systems/Blueprint/myCharacters/Enemy/AI/AM_BossDeath.AM_BossDeath"
        (:`then`
          (message `/Game/Systems/Blueprint/Interfaces/BPI_Win.FunctionWin` (`self.Player Character`))
          (`KismetSystemLibrary.Delay` 3.0)
          (`self.K2_DestroyActor`))))))

(fn `UserConstructionScript`)