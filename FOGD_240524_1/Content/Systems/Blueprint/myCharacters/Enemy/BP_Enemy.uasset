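; BP_Enemy is an enemy Blueprint that turns its mesh as it moves and tracks damage taken.
; Every tick, FacePlayer smoothly interpolates the mesh's world rotation toward the yaw of its velocity, so despite the name it follows movement direction rather than the player.
; AnyDamage subtracts damage from CurrentHealth and prints the result, with no death handling.
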(event `self.ReceiveTick`
  (params (DeltaSeconds :type "Float (single-precision)"))
  (`self.FacePlayer`))

(event `self.ReceiveBeginPlay`)

(event `FacePlayer`
  (bind _mesh (`self.Mesh`))
  (bind (_returnvalue_roll _returnvalue_pitch _returnvalue_yaw) (`KismetMathLibrary.BreakRotator` (`KismetMathLibrary.MakeRotFromX` (`self.GetVelocity`))))
  (`SceneComponent.K2_SetWorldRotation` _mesh (`KismetMathLibrary.RInterpTo` (`SceneComponent.K2_GetComponentRotation` _mesh) (`KismetMathLibrary.MakeRotator` 0.0 0.0 _returnvalue_yaw) (`GameplayStatics.GetWorldDeltaSeconds`) 2.0) false false))

(event `self.ReceiveAnyDamage`
  (params (Damage :type "Float (single-precision)") (DamageType :type "DamageType Object Reference") (InstigatedBy :type "Controller Object Reference") (DamageCauser :type "Actor Object Reference"))
  (bind _output_get (set `self.Current Health` (- (`self.Current Health`) Damage)))
  (`KismetSystemLibrary.PrintString` (`KismetStringLibrary.Conv_DoubleToString` _output_get)))

(fn `UserConstructionScript`)