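; BP_SnowyTree1 is a snowy tree actor that turns into a dead tree when a projectile hits it.
; When its StaticMesh begins overlapping a BP_Projectile, it spawns BP_DeadTree1 at its own location, clears its OverlappingActors array and destroys itself.
; A Box-based overlap query for projectiles remains in the graph but never runs.
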(event `self.StaticMesh.OnComponentBeginOverlap`
  (params (OverlappedComponent :type "PrimitiveComponent Object Reference") (OtherActor :type "Actor Object Reference") (OtherComp :type "PrimitiveComponent Object Reference") (OtherBodyIndex :type Integer) (bFromSweep :type Boolean) (SweepResult :type "HitResult Structure (by ref)"))
  (cast `/Game/Systems/Blueprint/BP_Projectile` OtherActor)
  (`|SpawnActorFromClass` "/Game/Systems/Blueprint/Decor/BP_DeadTree1.BP_DeadTree1_C" (`KismetMathLibrary.MakeTransform` (`self.K2_GetActorLocation`)) "Undefined" "MultiplyWithRoot" null null)
  (`KismetArrayLibrary.Array_Clear` (`self.Overlapping Actors`))
  (`self.K2_DestroyActor`))

(fn `UserConstructionScript`)